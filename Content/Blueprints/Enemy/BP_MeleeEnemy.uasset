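; Melee enemy character Blueprint that handles animation and health bar responses to combat events such as attacks, hits, blocks, finishers and death.
; Each event plays its montage unless already playing, and montage endings restore movement, signal attack completion or stop blocking.
; Hit reactions alternate left and right via FlipFlop, freeze movement, then roll a chance to start blocking.
; The health bar widget tracks HealthComponent and hides at zero.
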(event EventOnDamageReceivedEvent
  (bind _mesh (Variables|Character|GetMesh))
  (bind _mesh_2 (Variables|Character|GetMesh))
  (bind _returnvalue (Components|SkeletalMesh|GetAnimInstance _mesh))
  ;[0.01377 1 0] Damage Received
  (if (not (or (Animation|Montage|MontageIsPlaying _returnvalue "/Game/Animations/Enemy/AM_HitReactLeft.AM_HitReactLeft") (Animation|Montage|MontageIsPlaying _returnvalue "/Game/Animations/Enemy/AM_HitReactRight.AM_HitReactRight")))
    (Pawn|Components|CharacterMovement|SetMovementMode (Variables|Character|GetCharacterMovement) "MOVE_None" 0)
    (Utilities|FlowControl|FlipFlop
      (:A
        (Animation|Montage|PlayMontage _mesh_2 "/Game/Animations/Enemy/AM_HitReactLeft.AM_HitReactLeft"
          (:OnCompleted
            _)
          (:OnBlendOut
            _)
          (:OnInterrupted
            _)))
      (:B
        (Animation|Montage|PlayMontage _mesh_2 "/Game/Animations/Enemy/AM_HitReactRight.AM_HitReactRight"
          (:OnCompleted
            _)
          (:OnBlendOut
            _)
          (:OnInterrupted
            _))))
    (Pawn|Components|CharacterMovement|SetMovementMode (Variables|Character|GetCharacterMovement) "MOVE_Walking" 0)
    (if (< (Math|Random|RandomInteger 100) (Variables|Default|GetBlockChancePercentage))
      (Utilities|FlowControl|Delay 0.2)
      (Class|MeleeEnemy|StartBlocking))))

(event Collision|EventActorBeginOverlap
  (params (OtherActor :type Actor%20Object%20Reference)))

(event EventPlayAttackMontageEvent
  ;[1 0 0.004658] Attack
  (if (not (Animation|Montage|MontageIsPlaying (Components|SkeletalMesh|GetAnimInstance (Variables|Character|GetMesh)) "/Game/Animations/Enemy/AM_MeleeEnemyCombo.AM_MeleeEnemyCombo"))
    (Animation|Montage|PlayMontage (Variables|Character|GetMesh) "/Game/Animations/Enemy/AM_MeleeEnemyCombo.AM_MeleeEnemyCombo"
      (:OnCompleted
        _)
      (:OnBlendOut
        _)
      (:OnInterrupted
        _))
    (Class|BaseCharacter|OnAttackFinished)
    (Variables|/Script/Engine.CharacterMovementComponent|SetMaxWalkSpeed (Variables|Character|GetCharacterMovement) (Variables|Default|GetBaseMaxWalkSpeed))))

(event EventTick
  (params (DeltaSeconds :type Float%20%28single-precision%29)))

(event EventPlayDyingMontageEvent
  ;[0.01377 1 0] Damage Received
  (if (not (Animation|Montage|MontageIsPlaying (Components|SkeletalMesh|GetAnimInstance (Variables|Character|GetMesh)) "/Game/Animations/Enemy/AM_Die.AM_Die"))
    (Animation|Montage|PlayMontage (Variables|Character|GetMesh) "/Game/Animations/Enemy/AM_Die.AM_Die")))

(event EventOnAttackBlockedEvent
  ;[0 0.1036 1] Block
  (if (not (Animation|Montage|MontageIsPlaying (Components|SkeletalMesh|GetAnimInstance (Variables|Character|GetMesh)) "/Game/Animations/Enemy/AM_AttackBlockedReact.AM_AttackBlockedReact"))
    (Animation|Montage|PlayMontage (Variables|Character|GetMesh) "/Game/Animations/Enemy/AM_AttackBlockedReact.AM_AttackBlockedReact"
      (:OnCompleted
        _)
      (:OnBlendOut
        _)
      (:OnInterrupted
        _))
    (Variables|/Script/Engine.CharacterMovementComponent|SetMaxWalkSpeed (Variables|Character|GetCharacterMovement) (Variables|Default|GetBaseMaxWalkSpeed))))

(event EventDamageBlockedEvent
  ;[0 0.1036 1] Block
  (if (not (Animation|Montage|MontageIsPlaying (Components|SkeletalMesh|GetAnimInstance (Variables|Character|GetMesh)) "/Game/Animations/Enemy/AM_DamageBlocked.AM_DamageBlocked"))
    (Animation|Montage|PlayMontage (Variables|Character|GetMesh) "/Game/Animations/Enemy/AM_DamageBlocked.AM_DamageBlocked"
      (:OnCompleted
        _)
      (:OnBlendOut
        _)
      (:OnInterrupted
        _))
    (Class|MeleeEnemy|StopBlocking)))

(event EventUpdateHealthWidgetEvent
  (bind _healthbarwidget (Variables|Default|GetHealthBarWidget))
  (bind _healthcomponent (Variables|Default|GetHealthComponent))
  (bind _returnvalue (Class|HealthComponent|GetHealthPercent _healthcomponent))
  ;[0.01377 1 0] Damage Received
  (bind _aswbp_enemy_health_bar (Utilities|Casting|CastToWBP_EnemyHealthBar (UserInterface|GetWidget _healthbarwidget)))
  (if (<= _returnvalue 0.0)
    (Rendering|SetVisibility _healthbarwidget false false)
    (else
      (Progress|SetPercent (Variables|/Game/Widgets/WBP_EnemyHealthBar.WBP_EnemyHealthBar_C|GetHealthBar _aswbp_enemy_health_bar) _returnvalue))))

(event EventPlayFinisherMontageEventDefend
  ;[1 0 0.004658] Attack
  (if (not (Animation|Montage|MontageIsPlaying (Components|SkeletalMesh|GetAnimInstance (Variables|Character|GetMesh)) "/Game/Animations/Enemy/AM_FinisherDefend.AM_FinisherDefend"))
    (Pawn|Components|CharacterMovement|SetMovementMode (Variables|Character|GetCharacterMovement) "MOVE_None" 0)
    (Animation|Montage|PlayMontage (Variables|Character|GetMesh) "/Game/Animations/Enemy/AM_FinisherDefend.AM_FinisherDefend")))

(fn ConstructionScript)